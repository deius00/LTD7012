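; Player character for a 2D side-scrolling endless runner that auto-runs along +X, jumps on input and tracks distance traveled.
; Tick drains boots durability, drives movement and picks Paper2D flipbooks and facing from velocity.
; MyGameInstance event dispatchers deliver powerup hits, which raise durability and speed, and stub hits, which kill the player.
; Death, also triggered by worn-out boots, stops movement and broadcasts game over through the game instance.
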(event Custom|Event%20Powerup%20Collision
  ;[1 1 1] Bind to events
  (CallFunction|HandlePowerupCollision))

(event Custom|Event%20Stub%20Collision
  ;[1 1 1] Bind to events
  (CallFunction|PlayerDied)
  (Default|CallGameOverED (Variables|Default|GetCachedGameInstance)))

(event EventBeginPlay
  (Input|SetInputModeGameOnly (Game|GetPlayerController 0))
  ;[1 1 1] Cache MyGameInstance reference
  (bind _asmy_game_instance (Utilities|Casting|CastToMyGameInstance (Game|GetGameInstance)))
  (Variables|Default|SetCachedGameInstance _asmy_game_instance)
  (CallFunction|InitializePlayerState)
  ;[1 1 1] Bind to events
  (EventDispatchers|BindEventtoPowerupCollisionED (Variables|Default|GetCachedGameInstance) (delegate Custom|Event%20Powerup%20Collision))
  (EventDispatchers|BindEventtoStubCollisionED (Variables|Default|GetCachedGameInstance) (delegate Custom|Event%20Stub%20Collision)))

(event EventTick
  (params (DeltaSeconds :type Float%20%28single-precision%29))
  (if (Variables|Default|GetPlayerIsAlive)
    (CallFunction|UpdateBootsDurability DeltaSeconds)
    (CallFunction|UpdatePlayerPosition)
    (CallFunction|UpdateAnimation)
    (CallFunction|UpdateJumpState)
    (CallFunction|UpdateDistanceTraveled)
    (else
      (Sprite|SetFlipbook (Variables|Default|GetSprite) "/Game/Flipbooks/PlayerGameOver.PlayerGameOver"))))

(event Input|ActionEvents|InputActionJump
  (params (Key :type Key%20Structure :default "None"))
  (:Pressed
    (if (Variables|Default|GetPlayerIsAlive)
      ;[1 1 1] Handle jumping
      (Character|Jump)
      (Variables|Default|SetPlayerIsJumping true)))
  (:Released
    (Character|StopJumping)))

(fn ConstructionScript)

(fn InitializePlayerState
  ;[1 1 1] Set up player initial state
  (Variables|Default|SetPlayerIsAlive (Math|Conversions|ToBoolean(Integer) 1))
  (Variables|Default|SetMovementSpeedCurrent (Variables|Default|GetMovementSpeedInitial))
  (Variables|Default|SetBootsDurabilityCurrent (Variables|Default|GetBootsDurabilityInitial))
  (Variables|Default|SetPlayerInitialX (.X (Math|Vector|BreakVector (Transformation|GetWorldLocation (Variables|Collision|GetCapsuleComponent))))))

(fn GetBootsDurabilityNormalized
  (return (Math|Float|Clamp(Float) (/ (Variables|Default|GetBootsDurabilityCurrent) (Variables|Default|GetBootsDurabilityMax)))))

(fn UpdateBootsDurability
  (params (dt%20seconds :type Float%20%28single-precision%29))
  (bind _output_get (Variables|Default|SetBootsDurabilityCurrent (- (Variables|Default|GetBootsDurabilityCurrent) (* (LocalVariables|GetBootsDegradationPerSecond) dt%20seconds))))
  (if (not (> _output_get 0.0))
    (CallFunction|PlayerDied)))

(fn UpdatePlayerPosition
  ;[1 1 1] Move player right at every tick
  (Pawn|Input|AddMovementInput "1.000000, 0, 0" 1.0 false)
  (Variables|/Script/Engine.CharacterMovementComponent|SetMaxWalkSpeed (Variables|Character|GetCharacterMovement) (Variables|Default|GetMovementSpeedCurrent)))

(fn UpdateAnimation
  (bind _returnvalue (Transformation|GetVelocity))
  (bind _returnvalue_2 (Pawn|GetController))
  (bind _returnvalue_3 (Pawn|GetController))
  (bind _returnvalue_4 (Transformation|GetVelocity))
  (bind _sprite (Variables|Default|GetSprite))
  (bind _sprite_2 (Variables|Default|GetSprite))
  (bind _x (Math|Vector|BreakVector _returnvalue))
  (if (Variables|Default|GetPlayerIsJumping)
    ;[1 1 1] Jumping up, determine moving up or moving down
    ;;[1 1 1] Moving left or right
    (Math|Float|CompareFloat (.X (Math|Vector|BreakVector _returnvalue_4)) 0.0
      (:>
        ;;[1 1 1] Determine direction
        (Pawn|SetControlRotation _returnvalue_3 (Math|Rotator|MakeRotator 0.0 0.0 0.0)))
      (:<
        (Pawn|SetControlRotation _returnvalue_3 (Math|Rotator|MakeRotator 0.0 0.0 1.8e+02))))
    ;;[1 1 1] Moving up or down
    (Math|Float|CompareFloat (.Z (Math|Vector|BreakVector _returnvalue_4)) 0.0
      (:>
        (Sprite|SetFlipbook _sprite "/Game/Flipbooks/PlayerJump.PlayerJump"))
      (:<
        (Sprite|SetFlipbook _sprite "/Game/Flipbooks/PlayerFall.PlayerFall")))
    (else
      ;[1 1 1] Not jumping, determing if idle or moving
      (Math|Float|CompareFloat _x 0.0
        (:>
          (Pawn|SetControlRotation _returnvalue_2 (Math|Rotator|MakeRotator 0.0 0.0 0.0)))
        (:==
          _)
        (:<
          (Pawn|SetControlRotation _returnvalue_2 (Math|Rotator|MakeRotator 0.0 0.0 1.8e+02))))
      (Math|Float|CompareFloat (Math|Float|Absolute(Float) _x) 0.1
        (:>
          (Sprite|SetFlipbook _sprite_2 "/Game/Flipbooks/PlayerRun.PlayerRun"))
        (:<
          (Sprite|SetFlipbook _sprite_2 "/Game/Flipbooks/PlayerIdle.PlayerIdle"))))))

(fn UpdateJumpState
  (Math|Float|CompareFloat (.Z (Math|Vector|BreakVector (Transformation|GetVelocity))) 0.0
    (:==
      (Variables|Default|SetPlayerIsJumping false))))

(fn UpdateDistanceTraveled
  (Variables|Default|SetDistanceTraveled (/ (- (.X (Math|Vector|BreakVector (Transformation|GetWorldLocation (Variables|Collision|GetCapsuleComponent)))) (Variables|Default|GetPlayerInitialX)) 1e+02)))

(fn HandlePowerupCollision
  ;[1 1 1] Increase boots durability
  (Variables|Default|SetBootsDurabilityCurrent (Math|Float|Clamp(Float) (+ (Variables|Default|GetBootsDurabilityCurrent) (Math|Float|MakeLiteralFloat 1e+01)) 0.0 (Variables|Default|GetBootsDurabilityMax)))
  ;[1 1 1] Apply speed boost for player
  (Variables|Default|SetMovementSpeedCurrent (Math|Float|Clamp(Float) (+ (Variables|Default|GetMovementSpeedCurrent) (Math|Float|MakeLiteralFloat 5e+01)) 0.0 (Variables|Default|GetMovementSpeedMax))))

(fn PlayerDied
  (Variables|Default|SetPlayerIsAlive false)
  (Variables|Default|SetMovementSpeedCurrent 0.0)
  (Variables|/Script/Engine.CharacterMovementComponent|SetMaxWalkSpeed (Variables|Character|GetCharacterMovement) 0.0)
  (Default|CallGameOverED (Variables|Default|GetCachedGameInstance)))