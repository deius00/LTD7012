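; Boots powerup pickup that pulses in size while it sits in the level.
; Each tick, UpdateSpriteSize multiplies a scale modifier up or down and flips direction at upper and lower limits, producing a breathing effect.
; Overlapping the sphere collider fires the game instance's powerup collision dispatcher, plays a 2D sound and destroys the actor.
; BeginPlay, Tick and DoCleanup defer to the parent class.
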(event OnComponentBeginOverlap(SphereCollider)
  (params (OverlappedComponent :type Primitive%20Component%20Object%20Reference) (OtherActor :type Actor%20Object%20Reference) (OtherComp :type Primitive%20Component%20Object%20Reference) (OtherBodyIndex :type Integer) (bFromSweep :type Boolean) (SweepResult :type Hit%20Result%20Structure%20%28by%20ref%29))
  ;[1 1 1] Call global event dispatcher
  (Default|CallPowerupCollisionED (Variables|Default|GetCachedGameInstance))
  (Audio|PlaySound2D "/Game/Sounds/BootsPowerup.BootsPowerup" 1.0 1.0 0.0 0 0)
  (Actor|DestroyActor))

(event EventBeginPlay
  (|CallParentFunction))

(event EventTick
  (params (DeltaSeconds :type Float%20%28single-precision%29))
  (|CallParentFunction DeltaSeconds)
  (CallFunction|UpdateSpriteSize))

(fn ConstructionScript)

(fn UpdateSpriteSize
  (if (Variables|Default|GetIsScaleGrowing)
    ;[1 1 1] Grow scale
    (bind _output_get (Variables|Default|SetCurrentScaleModifier (* (Variables|Default|GetCurrentScaleModifier) 1.01)))
    ;[1 1 1] Check to stop growing
    (if (> _output_get 1.25)
      (Variables|Default|SetIsScaleGrowing false))
    (else
      ;[1 1 1] Shrink scale
      (bind _output_get_2 (Variables|Default|SetCurrentScaleModifier (* (Variables|Default|GetCurrentScaleModifier) 0.99)))
      ;[1 1 1] Check to stop shrinking
      (if (< _output_get_2 0.75)
        (Variables|Default|SetIsScaleGrowing true))))
  (Transformation|SetActorScale3D (Math|Conversions|ToVector(Float) (Variables|Default|GetCurrentScaleModifier))))

(fn DoCleanup
  (|CallParentFunction))