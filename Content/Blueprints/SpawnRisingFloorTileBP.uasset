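; SpawnRisingFloorTileBP is a floor tile for a run mode that triggers the next tile as the hero passes through.
; When HeroBP overlaps EndTrigger, it calls AddFloorTile on RunGameMode, then destroys itself after that game mode's TimeUntilTileDespawn delay.
; GetAttachTransform exposes the AttachPoint world transform.
; Nothing in its graphs implements the rising motion the name suggests.
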(event OnComponentBeginOverlap(EndTrigger)
  (params (OverlappedComponent :type Primitive%20Component%20Object%20Reference) (OtherActor :type Actor%20Object%20Reference) (OtherComp :type Primitive%20Component%20Object%20Reference) (OtherBodyIndex :type Integer) (bFromSweep :type Boolean) (SweepResult :type Hit%20Result%20Structure%20%28by%20ref%29))
  (Utilities|Casting|CastToHeroBP OtherActor)
  (bind _asrun_game_mode (Utilities|Casting|CastToRunGameMode (Game|GetGameMode)))
  (Default|AddFloorTile _asrun_game_mode)
  (Utilities|FlowControl|Delay (Variables|/Game/RunGameMode.RunGameMode_C|GetTimeUntilTileDespawn _asrun_game_mode))
  (Actor|DestroyActor))

(event EventBeginPlay)

(event Collision|EventActorBeginOverlap
  (params (OtherActor :type Actor%20Object%20Reference)))

(event EventTick
  (params (DeltaSeconds :type Float%20%28single-precision%29)))

(fn ConstructionScript)

(fn GetAttachTransform
  (return (Transformation|GetWorldTransform (Variables|Default|GetAttachPoint))))