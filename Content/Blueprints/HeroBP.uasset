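; Player-controlled 2D side-scrolling hero character that runs along the X axis and jumps.
; Left and right axis events add movement input and flip control rotation yaw to face the direction of travel.
; Both axis events also call UpdateAnimation, which picks the idle, run or jump flipbook from velocity and an IsJumping flag.
; Jump input sets that flag, and UpdateAnimation clears it when vertical velocity is zero.
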(event Custom|Update%20Animation
  ;[1 1 1] Update animation
  (if (Variables|Default|GetbIsJumping)
    ;;[1 1 1] Check jump state
    (Math|Float|CompareFloat (.Z (Math|Vector|BreakVector (Transformation|GetVelocity))) 0.0
      (:>
        _)
      (:==
        (Variables|Default|SetbIsJumping false))
      (:<
        _))
    (Sprite|SetFlipbook (Variables|Default|GetSprite) "/Game/Flipbooks/HeroJump.HeroJump")
    (else
      (Math|Float|CompareFloat (Math|Float|Absolute(Float) (.X (Math|Vector|BreakVector (Transformation|GetVelocity)))) 0.0
        (:>
          (Sprite|SetFlipbook (Variables|Default|GetSprite) "/Game/Flipbooks/HeroRun.HeroRun"))
        (:==
          (Sprite|SetFlipbook (Variables|Default|GetSprite) "/Game/Flipbooks/HeroIdle.HeroIdle"))))))

(event EventBeginPlay
  (Input|SetInputModeGameOnly (Game|GetPlayerController 0)))

(event Collision|EventActorBeginOverlap
  (params (OtherActor :type Actor%20Object%20Reference)))

(event EventTick
  (params (DeltaSeconds :type Float%20%28single-precision%29)))

(event Input|ActionEvents|InputActionJump
  (params (Key :type Key%20Structure :default "None"))
  ;[1 1 1] Handle jumping
  (:Pressed
    (Character|Jump)
    (Variables|Default|SetbIsJumping true))
  (:Released
    (Character|StopJumping)))

(event Input|AxisEvents|InputAxisMoveAxisRight
  (params (AxisValue :type Float%20%28single-precision%29))
  ;[1 1 1] Handle movement
  (Pawn|Input|AddMovementInput "1.000000, 0, 0" AxisValue false)
  (CallFunction|UpdateAnimation)
  (Math|Float|CompareFloat AxisValue 0.0
    (:>
      ;;[1 1 1] Facing right
      (Pawn|SetControlRotation (Game|GetPlayerController 0) (Math|Rotator|MakeRotator 0.0 0.0 0.0)))))

(event Input|AxisEvents|InputAxisMoveAxisLeft
  (params (AxisValue :type Float%20%28single-precision%29))
  ;[1 1 1] Handle movement
  (Pawn|Input|AddMovementInput "-1.000000, 0, 0" AxisValue false)
  (CallFunction|UpdateAnimation)
  (Math|Float|CompareFloat AxisValue 0.0
    (:>
      ;;[1 1 1] Facing left
      (Pawn|SetControlRotation (Game|GetPlayerController 0) (Math|Rotator|MakeRotator 0.0 0.0 1.8e+02)))))

(fn ConstructionScript)