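; Descending track tile Blueprint, a child of a parent tile class, that supplies the attach point for the next spawn and hosts a boots powerup.
; GetSpawnPoint returns the AttachPoint transform, and SpawnPowerup places an InteractableBootsBP at PowerupSpawnPoint.
; Overlapping EndTrigger calls the DespawnTile event dispatcher with this tile.
; Stub and prop spawning defer to the parent, while cleanup also destroys the powerup and stub instances.
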(event OnComponentBeginOverlap(EndTrigger)
  (params (OverlappedComponent :type Primitive%20Component%20Object%20Reference) (OtherActor :type Actor%20Object%20Reference) (OtherComp :type Primitive%20Component%20Object%20Reference) (OtherBodyIndex :type Integer) (bFromSweep :type Boolean) (SweepResult :type Hit%20Result%20Structure%20%28by%20ref%29))
  (Default|CallDespawnTileED self))

(event EventBeginPlay
  (|CallParentFunction))

(event EventTick
  (params (DeltaSeconds :type Float%20%28single-precision%29)))

(fn ConstructionScript)

(fn GetSpawnPoint
  (|CallParentFunction)
  (return (Transformation|GetWorldTransform (Variables|Default|GetAttachPoint))))

(fn SpawnPowerup
  (|CallParentFunction)
  (bind _returnvalue (Game|SpawnActorfromClass "/Game/Blueprints/Collectibles/InteractableBootsBP.InteractableBootsBP_C" (Transformation|GetWorldTransform (Variables|Default|GetPowerupSpawnPoint)) "Undefined" 0 0))
  (Variables|Default|SetPowerupInstance _returnvalue))

(fn SpawnStubs
  (|CallParentFunction))

(fn SpawnProps
  (|CallParentFunction))

(fn DoCleanup
  (bind _powerupinstance (Variables|Default|GetPowerupInstance))
  (bind _stubinstance (Variables|Default|GetStubInstance))
  (|CallParentFunction)
  ;[1 1 1] Despawn powerup if valid
  (Utilities|IsValid _powerupinstance
    (:Is%20Valid
      (Actor|DestroyActor _powerupinstance))
    (:Is%20Not%20Valid
      _))
  ;[1 1 1] Despawn stubs if valid
  (Utilities|IsValid _stubinstance
    (:Is%20Valid
      (Actor|DestroyActor _stubinstance))))