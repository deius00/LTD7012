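; TileFlatBP is a flat track tile that extends a parent tile with its own pickup, obstacle and prop spawning.
; It supplies its attach point transform as the spawn point and broadcasts a despawn dispatcher when anything overlaps its end trigger.
; Spawn overrides place a boots powerup, a stub at one of two random points, and randomly rescale a tree.
; Cleanup destroys the stored powerup and stub instances.
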(event OnComponentBeginOverlap(EndTrigger)
  (params (OverlappedComponent :type Primitive%20Component%20Object%20Reference) (OtherActor :type Actor%20Object%20Reference) (OtherComp :type Primitive%20Component%20Object%20Reference) (OtherBodyIndex :type Integer) (bFromSweep :type Boolean) (SweepResult :type Hit%20Result%20Structure%20%28by%20ref%29))
  (Default|CallDespawnTileED self))

(event EventBeginPlay
  (|CallParentFunction))

(event EventTick
  (params (DeltaSeconds :type Float%20%28single-precision%29)))

(fn ConstructionScript)

(fn GetSpawnPoint
  ;[1 1 1] Get spawn attachment point for tile
  (|CallParentFunction)
  (return (Transformation|GetWorldTransform (Variables|Default|GetAttachPoint))))

(fn SpawnPowerup
  (|CallParentFunction)
  ;[1 1 1] Randomize Boots spawn
  (bind _returnvalue (Game|SpawnActorfromClass "/Game/Blueprints/Interactables/InteractableBootsBP.InteractableBootsBP_C" (Transformation|GetWorldTransform (Variables|Default|GetPowerupSpawnPoint)) "Undefined" 0 0))
  (Variables|Default|SetPowerupInstance _returnvalue))

(fn SpawnStubs
  (|CallParentFunction)
  (if (> (Math|Random|RandomInteger 2) 0)
    (bind _returnvalue (Game|SpawnActorfromClass "/Game/Blueprints/Interactables/InteractableStubBP.InteractableStubBP_C" (Transformation|GetWorldTransform (Variables|Default|GetStubSpawnPoint1)) "Undefined" 0 0))
    (Variables|Default|SetStubInstance _returnvalue)
    (else
      (bind _returnvalue_2 (Game|SpawnActorfromClass "/Game/Blueprints/Interactables/InteractableStubBP.InteractableStubBP_C" (Transformation|GetWorldTransform (Variables|Default|GetStubSpawnPoint2)) "Undefined" 0 0))
      (Variables|Default|SetStubInstance _returnvalue_2))))

(fn SpawnProps
  (|CallParentFunction)
  ;[1 1 1] Randomize BigPropTree size
  (if (> (Math|Random|RandomInteger 10) 3)
    (Transformation|SetWorldScale3D (Variables|Default|GetBigPropTree) (Math|Conversions|ToVector(Float) 0.6))))

(fn DoCleanup
  (bind _powerupinstance (Variables|Default|GetPowerupInstance))
  (bind _stubinstance (Variables|Default|GetStubInstance))
  (|CallParentFunction)
  ;[1 1 1] Despawn powerup if valid
  (Utilities|IsValid _powerupinstance
    (:Is%20Valid
      (Actor|DestroyActor _powerupinstance))
    (:Is%20Not%20Valid
      _))
  ;[1 1 1] Despawn stubs if valid
  (Utilities|IsValid _stubinstance
    (:Is%20Valid
      (Actor|DestroyActor _stubinstance))))